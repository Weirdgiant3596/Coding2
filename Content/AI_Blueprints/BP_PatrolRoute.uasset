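; BP_PatrolRoute is a patrol route actor that supplies world-space waypoints from the points of its Spline.
; GetPatrolPointLocation steps PatrolIndex by Direction and returns that point's location, with branches meant to reverse Direction at the route's ends.
; The first branch is fixed to true, so Direction always becomes -1 and the lower-bound reversal never runs.
; The end-of-spline comparisons and a direction-flip node are left unconnected.
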(event EventBeginPlay)

(event Collision|EventActorBeginOverlap
  (params (OtherActor :type Actor%20Object%20Reference)))

(event EventTick
  (params (DeltaSeconds :type Float%20%28single-precision%29)))

(fn ConstructionScript)

(fn GetPatrolPointLocation
  (Variables|Default|SetPatrolIndex (+ (Variables|Default|GetPatrolIndex) (Variables|Default|GetDirection)))
  (if true
    (Variables|Default|SetDirection -1)
    (return (Spline|GetLocationatSplinePoint (Variables|Default|GetSpline) (Variables|Default|GetPatrolIndex) "World"))
    (elif (<= (Variables|Default|GetPatrolIndex) 0)
      (Variables|Default|SetDirection 1)
      (else
        (return (Spline|GetLocationatSplinePoint (Variables|Default|GetSpline) (Variables|Default|GetPatrolIndex) "World"))))))