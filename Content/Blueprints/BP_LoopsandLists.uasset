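; BP_LoopsandLists is a demonstration Blueprint that prints on-screen messages to show loop types and array access.
; BeginPlay starts DelayLoop, a self-calling event that uses a one-second Delay and a DoN node to repeat a limited number of times, running StartForLoop each pass.
; StartForLoop prints indices colored from a color array.
; The while-loop countdown and for-each color events are defined but not called here.
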(event Custom|Delay%20Loop
  (Development|PrintText (Utilities|Text|FormatText "This has run {count} times." (stale _counter)))
  (Utilities|FlowControl|Delay 1.0)
  (bind _counter (Utilities|FlowControl|DoN 20)
    (:Exit
      (CallFunction|StartforLoop)
      (CallFunction|DelayLoop))))

(event Custom|StartForLoop
  (bind _array (Utilities|Array|MakeArray "(R=0.000000,G=0.000000,B=0.000000,A=1.000000)" "(R=0.802669,G=0.000000,B=1.000000,A=1.000000)" "(R=0.003812,G=1.000000,B=0.989578,A=1.000000)" "(R=1.000000,G=0.897924,B=0.000000,A=1.000000)" "(R=0.123097,G=0.000000,B=1.000000,A=1.000000)" "(R=0.104022,G=1.000000,B=0.000126,A=1.000000)"))
  (for _index (range 0 (- (Utilities|Array|Length _array) 1) 2)
    (Development|PrintText (Utilities|Text|FormatText "This is Index # {index}." _index) true true (Utilities|Array|Get(acopy) _array _index))))

(event Custom|StartWhileLoop
  (while (> (Variables|Default|GetWhileLoopCounter) 0)
    (Development|PrintText (Utilities|Text|FormatText "There are {uses} more uses in this loop." (Variables|Default|GetWhileLoopCounter)) true true "(R=1.000000,G=0.206779,B=0.652174,A=1.000000)")
    (Math|Integer|DecrementInt (Variables|Default|GetWhileLoopCounter)))
  (Variables|Default|SetWhileLoopCounter 10))

(event Custom|StartForEachLoop
  (for (_array_element _array_index) (Utilities|Array|MakeArray "(R=0.000000,G=0.000000,B=0.000000,A=1.000000)" "(R=0.802669,G=0.000000,B=1.000000,A=1.000000)" "(R=0.003812,G=1.000000,B=0.989578,A=1.000000)" "(R=1.000000,G=0.897924,B=0.000000,A=1.000000)" "(R=0.123097,G=0.000000,B=1.000000,A=1.000000)" "(R=0.104022,G=1.000000,B=0.000126,A=1.000000)")
    (Development|PrintText (Utilities|Text|FormatText "This is Index # {index}." _array_index) true true _array_element)))

(event EventBeginPlay
  (Development|PrintString "Loops and Lists BP Exists")
  (CallFunction|DelayLoop))

(event Collision|EventActorBeginOverlap
  (params (OtherActor :type Actor%20Object%20Reference)))

(event EventTick
  (params (DeltaSeconds :type Float%20%28single-precision%29)))

(fn ConstructionScript)