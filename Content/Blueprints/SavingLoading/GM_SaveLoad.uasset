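; Game mode that handles saving and loading of player stats and per-level state, running both loads on BeginPlay.
; Player stats use the "PlayerSave" slot; level state uses a slot named after the current level, and missing saves get fresh objects.
; Loading re-collects saved coins and targets character Stamina, though that cast is fed the player controller rather than the pawn.
; Separate events write both save objects back to their slots.
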(event Custom|Load%20Player%20Stats
  (bind _returnvalue (SaveGame|DoesSaveGameExist "PlayerSave"))
  (if _returnvalue
    (bind _returnvalue_2 (SaveGame|LoadGamefromSlot "PlayerSave"))
    (bind _assg_player_stats (Utilities|Casting|CastToSG_PlayerStats _returnvalue_2))
    (Variables|Default|SetSG_PlayerStats _assg_player_stats)
    (bind _asbp_third_person_character (Utilities|Casting|CastToBP_ThirdPersonCharacter (Game|GetPlayerController 0)))
    (Variables|/Game/ThirdPerson/Blueprints/BP_ThirdPersonCharacter.BP_ThirdPersonCharacter_C|SetStamina _asbp_third_person_character (Variables|/Game/Blueprints/SavingLoading/SG_PlayerStats.SG_PlayerStats_C|GetStamina (Variables|Default|GetSG_PlayerStats)))
    (Development|PrintString "Player Stats have been loaded" true true "(R=1.000000,G=0.464378,B=0.062500,A=1.000000)" 8.0)
    (else
      (bind _returnvalue_3 (SaveGame|CreateSaveGameObject "/Game/Blueprints/SavingLoading/SG_PlayerStats.SG_PlayerStats_C"))
      (Variables|Default|SetSG_PlayerStats _returnvalue_3))))

(event Custom|Save%20Player%20Stats
  (bind _returnvalue (SaveGame|SaveGametoSlot (Variables|Default|GetSG_PlayerStats) "PlayerSave"))
  (if _returnvalue
    (Development|PrintText "PLayer Stats Written to Save Game")
    (else
      (Development|PrintText "Plyer Stats Could NOt be Written to Save Game File"))))

(event Custom|Save%20Level%20State%20to%20File
  (bind _returnvalue (Game|GetCurrentLevelName true))
  (bind _returnvalue_2 (SaveGame|SaveGametoSlot (Variables|Default|GetSG_LevelState) _returnvalue))
  (if _returnvalue_2
    (Development|PrintText "Level State Saved" true true "(R=0.005741,G=0.432292,B=0.041131,A=1.000000)" 5.0)
    (else
      (Development|PrintText "Failed to Save" true true "(R=0.591304,G=0.000000,B=0.000000,A=1.000000)" 5.0))))

(event Custom|Load%20Level%20State%20From%20File
  (bind _returnvalue (Game|GetCurrentLevelName true))
  (bind _returnvalue_2 (SaveGame|DoesSaveGameExist _returnvalue))
  (if _returnvalue_2
    (bind _returnvalue_3 (SaveGame|LoadGamefromSlot _returnvalue))
    (bind _assg_level_state (Utilities|Casting|CastToSG_LevelState _returnvalue_3)
      (:then
        (Variables|Default|SetSG_LevelState _assg_level_state)
        (Development|PrintText "Loaded Existing level state")
        (for _array_element (Variables|/Game/Blueprints/SavingLoading/SG_LevelState.SG_LevelState_C|GetCollectedCoins (Variables|Default|GetSG_LevelState))
          (Utilities|IsValid _array_element
            (:Is%20Valid
              (Default|CollectThyself _array_element)))))
      (:CastFailed
        (Development|PrintText "cast failed")))
    (else
      (bind _returnvalue_4 (SaveGame|CreateSaveGameObject "/Game/Blueprints/SavingLoading/SG_LevelState.SG_LevelState_C"))
      (Variables|Default|SetSG_LevelState _returnvalue_4)
      (Development|PrintText "new game for level state has been created"))))

(event EventBeginPlay
  (Development|PrintString "Loading the SaveLoad Game Mode" true true "(R=1.000000,G=0.464378,B=0.062500,A=1.000000)")
  (CallFunction|LoadPlayerStats)
  (CallFunction|LoadLevelStatefromFile))

(event EventTick
  (params (DeltaSeconds :type Float%20%28single-precision%29)))

(fn ConstructionScript)