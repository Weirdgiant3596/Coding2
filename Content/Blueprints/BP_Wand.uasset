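; BP_Wand is a held item that can be picked up and dropped, with red and green lights acting as toggleable spells.
; UsePrimary and UseSecondary each print a debug message and flip their light on or off through a FlipFlop.
; Pickup snaps the wand to the BPI_ItemSocket socket on the given skeletal mesh and disables its box collision.
; Drop detaches it and resets its location, without re-enabling collision.
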(event EventBeginPlay)

(event Collision|EventActorBeginOverlap
  (params (OtherActor :type Actor%20Object%20Reference)))

(event EventTick
  (params (DeltaSeconds :type Float%20%28single-precision%29)))

(event EventPickup
  (params (Skeletal%20Mesh :type Skeletal%20Mesh%20Component%20Object%20Reference))
  (Development|PrintText "This flashlight is getting picked up.")
  (Transformation|AttachComponentToComponent Skeletal%20Mesh "BPI_ItemSocket" "SnapToTarget" "SnapToTarget" "SnapToTarget" true)
  (Collision|SetCollisionEnabled (Variables|Default|GetBox) "NoCollision"))

(event EventUsePrimary
  (bind _redlight (Variables|Default|GetRedLight))
  (Development|PrintText "Toggle Red Spell")
  (Utilities|FlowControl|FlipFlop
    (:A
      (Rendering|Components|Light|SetIntensity _redlight 0.0))
    (:B
      (Rendering|Components|Light|SetIntensity _redlight 4e+02))))

(event EventDrop
  (Transformation|DetachFromActor "KeepRelative" "KeepRelative" "KeepRelative")
  (Transformation|SetActorRelativeLocation (Transformation|GetActorLocation)))

(event EventUseSecondary
  (bind _greenlight (Variables|Default|GetGreenLight))
  (Development|PrintText "Toggle Green Spell")
  (Utilities|FlowControl|FlipFlop
    (:A
      (Rendering|Components|Light|SetIntensity _greenlight 0.0))
    (:B
      (Rendering|Components|Light|SetIntensity _greenlight 4e+02))))

(fn ConstructionScript)