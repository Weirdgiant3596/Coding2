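; BP_Spinner is a holdable item that can be picked up, dropped and used to change the look of its Spinner component.
; Pickup prints a flashlight message, snaps the item to the BPI_ItemSocket socket on the given skeletal mesh and disables Box collision.
; Drop detaches it at its current location without restoring collision.
; Primary and secondary use each flip-flop the Spinner between its own metallic material and the basic shape material.
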(event EventBeginPlay)

(event Collision|EventActorBeginOverlap
  (params (OtherActor :type Actor%20Object%20Reference)))

(event EventTick
  (params (DeltaSeconds :type Float%20%28single-precision%29)))

(event EventPickup
  (params (Skeletal%20Mesh :type Skeletal%20Mesh%20Component%20Object%20Reference))
  (Development|PrintText "This flashlight is getting picked up.")
  (Transformation|AttachComponentToComponent Skeletal%20Mesh "BPI_ItemSocket" "SnapToTarget" "SnapToTarget" "SnapToTarget" true)
  (Collision|SetCollisionEnabled (Variables|Default|GetBox) "NoCollision"))

(event EventUsePrimary
  (Utilities|FlowControl|FlipFlop
    (:A
      (Rendering|Material|SetMaterial (Variables|Default|GetSpinner) 0 "/DatasmithContent/Materials/FBXImporter/VRED/BrushedMetal.BrushedMetal"))
    (:B
      (Rendering|Material|SetMaterial (Variables|Default|GetSpinner) 0 "/Engine/BasicShapes/BasicShapeMaterial.BasicShapeMaterial"))))

(event EventDrop
  (Transformation|DetachFromActor "KeepRelative" "KeepRelative" "KeepRelative")
  (Transformation|SetActorRelativeLocation (Transformation|GetActorLocation)))

(event EventUseSecondary
  (Utilities|FlowControl|FlipFlop
    (:A
      (Rendering|Material|SetMaterial (Variables|Default|GetSpinner) 0 "/DatasmithContent/Materials/FBXImporter/VRED/MetallicCarpaint.MetallicCarpaint"))
    (:B
      (Rendering|Material|SetMaterial (Variables|Default|GetSpinner) 0 "/Engine/BasicShapes/BasicShapeMaterial.BasicShapeMaterial"))))

(fn ConstructionScript)