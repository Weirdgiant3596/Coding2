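; Spawn manager that populates the level with randomized BP_AiMoveTo enemies at BP_SpawnEnemyPoint locations.
; On BeginPlay it gathers every spawn point, prints their count, and spawns an AI at each with a 75% chance.
; Each spawned AI gets a random name on its text render, plus a random material and skeletal mesh.
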(event EventBeginPlay
  (bind _outactors (Actor|GetAllActorsOfClass "/Game/Blueprints/BP_SpawnEnemyPoint.BP_SpawnEnemyPoint_C")) ; Find all actors that are BP_SpawnEnemyPoints
  (Development|PrintText (Utilities|Text|FormatText "There are {count} Spawn points in the level." (Utilities|Array|Length _outactors)))
  (for _array_element _outactors
    (if (Math|Random|RandomBoolwithWeight 0.75)
      (bind _returnvalue (Game|SpawnActorfromClass "/Game/AI_Blueprints/BP_AiMoveTo.BP_AiMoveTo_C" (Transformation|GetActorTransform _array_element) "Undefined" "MultiplyWithRoot" _array_element 0))
      (Rendering|Components|TextRender|SetText (Variables|/Game/AI_Blueprints/BP_AiMoveTo.BP_AiMoveTo_C|GetTextRender _returnvalue) (.OutItem (Utilities|Array|Random (Utilities|Array|MakeArray "Mary" "Rose" "Iktor" "Rupor" "Len" "Hel"))))
      (Rendering|Material|SetMaterial (Variables|/Script/Engine.Character|GetMesh _returnvalue) 0 (.OutItem (Utilities|Array|Random (Utilities|Array|MakeArray "/DatasmithContent/Materials/AliasReference.AliasReference" "/Engine/VREditor/UI/ArrowMaterial.ArrowMaterial" "/AnimationSharing/AnimSharingGreen.AnimSharingGreen" "/DatasmithContent/Materials/FBXImporter/VRED/BrushedMetal.BrushedMetal" "/Engine/TemplateResources/MI_Template_BaseBlue_Metal.MI_Template_BaseBlue_Metal" "/DatasmithContent/Materials/FBXImporter/DeltaGenReferenceClearCoat.DeltaGenReferenceClearCoat"))))
      (Components|SkeletalMesh|SetSkeletalMeshAsset (Variables|/Script/Engine.Character|GetMesh _returnvalue) (.OutItem (Utilities|Array|Random (Utilities|Array|MakeArray (Components|SkeletalMesh|GetSkeletalMeshAsset (Variables|/Script/Engine.Character|GetMesh _returnvalue)) "/Game/SCK_Casual01/Mannequin/Character/Mesh/SK_Mannequin.SK_Mannequin" "/ControlRigModules/Modules/Meshes/SKM_Dragon_Template.SKM_Dragon_Template" "/Game/Characters/Mannequins/Meshes/SKM_Quinn_Simple.SKM_Quinn_Simple" "/Game/SCK_Casual01/Models/Premade_Characters/MESH_PC_01.MESH_PC_01")))))))

(event Collision|EventActorBeginOverlap
  (params (OtherActor :type Actor%20Object%20Reference)))

(event EventTick
  (params (DeltaSeconds :type Float%20%28single-precision%29)))

(fn ConstructionScript)